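; Enemy spawner portal that the player can destroy by colliding with it.
; It spawns a slime character just above itself on BeginPlay and on a looping timer.
; Player hits on its capsule subtract damage with a one-second cooldown, then destroy it once remaining health cannot survive another hit.
; Tick pushes the health ratio to the health bar widget.
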(event OnComponentHit(CapsuleComponent)
  (params (HitComponent :type Primitive%20Component%20Object%20Reference) (OtherActor :type Actor%20Object%20Reference) (OtherComp :type Primitive%20Component%20Object%20Reference) (NormalImpulse :type Vector :default "0, 0, 0") (Hit :type Hit%20Result%20Structure%20%28by%20ref%29))
  (if (Variables|Default|GetCanBeHit)
    (if (== OtherActor (Game|Player|GetPlayerPawn 0))
      (Variables|Default|SetCanBeHit false)
      (Variables|Default|SetHealth (- (Variables|Default|GetHealth) (Variables|Default|GetDamage)))
      (if (<= (- (Variables|Default|GetHealth) (Variables|Default|GetDamage)) 0.0)
        (Actor|DestroyActor)
        (else
          (Utilities|FlowControl|Delay 1.0)
          (Variables|Default|SetCanBeHit true))))))

(event EventBeginPlay
  (CallFunction|SpawnEnemy)
  (Utilities|Time|SetTimerbyFunctionName 0 "SpawnEnemy" (Variables|Default|GetTime) true))

(event Collision|EventActorBeginOverlap
  (params (OtherActor :type Actor%20Object%20Reference)))

(event EventTick
  (params (DeltaSeconds :type Float%20%28single-precision%29))
  (bind _ashealth_bp (Utilities|Casting|CastToHealth_BP (UserInterface|GetWidget (Variables|Default|GetHealthBar))))
  (Progress|SetPercent (Variables|/Game/Blueprints/Health_BP.Health_BP_C|GetHealthBar _ashealth_bp) (/ (Variables|Default|GetHealth) (Variables|Default|GetMaxHealth))))

(fn ConstructionScript)

(fn SpawnEnemy
  (Game|SpawnActorfromClass "/Game/Blueprints/SlimeCharacter_BP.SlimeCharacter_BP_C" (Math|Conversions|ToTransform(Vector) (+ (Transformation|GetActorLocation self) "0.000000,0.000000,10.000000")) "AlwaysSpawn" "MultiplyWithRoot" 0 0))