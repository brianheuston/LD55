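; Slime enemy character that hops toward the player and loses health when the player bumps into it.
; A looping timer started on BeginPlay launches it horizontally along the direction to the player every second.
; Capsule hits from the player subtract Damage, then either destroy the slime at zero health or briefly block further hits.
; Tick pushes the health ratio into its Health_BP widget's progress bar.
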(event OnComponentHit(CapsuleComponent)
  (params (HitComponent :type Primitive%20Component%20Object%20Reference) (OtherActor :type Actor%20Object%20Reference) (OtherComp :type Primitive%20Component%20Object%20Reference) (NormalImpulse :type Vector :default "0, 0, 0") (Hit :type Hit%20Result%20Structure%20%28by%20ref%29))
  (if (Variables|Default|GetCanBeHit)
    (if (== OtherActor (Game|GetPlayerCharacter 0))
      (Variables|Default|SetCanBeHit false)
      (bind _output_get (Variables|Default|SetHealth (- (Variables|Default|GetHealth) (Variables|Default|GetDamage))))
      (if (<= _output_get 0.0)
        (Actor|DestroyActor)
        (else
          (Utilities|FlowControl|Delay 1.0)
          (Variables|Default|SetCanBeHit true))))))

(event EventBeginPlay
  (CallFunction|Startup))

(event Collision|EventActorBeginOverlap
  (params (OtherActor :type Actor%20Object%20Reference)))

(event EventTick
  (params (DeltaSeconds :type Float%20%28single-precision%29))
  (bind _ashealth_bp (Utilities|Casting|CastToHealth_BP (UserInterface|GetWidget (Variables|Default|GetHealthBar))))
  (Progress|SetPercent (Variables|/Game/Blueprints/Health_BP.Health_BP_C|GetHealthBar _ashealth_bp) (/ (Variables|Default|GetHealth) (Variables|Default|GetMaxHealth))))

(fn ConstructionScript)

(fn SlimeJump
  (Character|LaunchCharacter (* (Math|Vector|Normalize (- (Transformation|GetActorLocation (Game|GetPlayerCharacter 0)) (Transformation|GetActorLocation))) "500.000000,500.000000,0.000000") false false))

(fn Startup
  (Utilities|Time|SetTimerbyFunctionName 0 "SlimeJump" 1.0 true))